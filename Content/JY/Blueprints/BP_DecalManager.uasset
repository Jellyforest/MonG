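; Manager actor that fades every DecalActor in the level in at game start and out on the IA_Quit input.
; BeginPlay caches all decal actors and runs DecalInitialize, which fades them in and sets IsGameReady.
; IA_Quit triggers DecalAllFadeReady once, clearing that flag; decals fade out without being destroyed.
; Re-initialization at an end condition is an unwired TODO, as is an EnableInput call.
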(event `self.ReceiveBeginPlay`
  (bind _outactors (`GameplayStatics.GetAllActorsOfClass` "/Script/Engine.DecalActor"))
  (set `self.MyDecals` _outactors)
  (`self.DecalInitialize`)
  (set `self.isGameReady` true))

(event `DecalAllFadeReady`
  (for _array_element (`self.MyDecals`)
    (bind _decal (`DecalActor.Decal` _array_element))
    (`DecalComponent.SetFadeIn` _decal 0.0 0.0)
    (`DecalComponent.SetFadeOut` _decal 0.2 (`DecalComponent.GetFadeDuration` _decal) false)))

(event `DecalInitialize`
  (for _array_element (`self.MyDecals`)
    (bind _decal (`DecalActor.Decal` _array_element))
    (`DecalComponent.SetFadeOut` _decal 0.0 (`DecalComponent.GetFadeDuration` _decal) false)
    (`DecalComponent.SetFadeIn` _decal 0.1 1.0))
  (if (not (`self.isGameReady`))
    (set `self.isGameReady` true)))

(event `EnhancedInput|/Game/JY/Input/IA_Quit`
  (params (ActionValue :type Boolean) (ElapsedSeconds :type "Float (double-precision)") (TriggeredSeconds :type "Float (double-precision)") (InputAction :type "InputAction Object Reference" :default "/Game/JY/Input/IA_Quit.IA_Quit"))
  (:`Started`
    (if (`self.isGameReady`)
      (`self.DecalAllFadeReady`)
      (set `self.isGameReady` false))))

(fn `UserConstructionScript`)