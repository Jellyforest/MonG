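; BP_DustStrollSpawner_Child is a dust spawner meant to wander between random move points, firing dust at each one.
; BeginPlay picks a random index into MovePoint0.
; Each Tick, it calls the Fire function and picks a new random target once within one unit of the current one.
; Otherwise it steps along the normalized direction, but MoveSpeed0 is multiplied by zero rather than DeltaSeconds, so that step is zero.
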(event `self.ReceiveBeginPlay`
  ;[1 1 1] 무브포인트를 랜덤으로 왔다갔다 했으면 좋겠다
  (`parent.ReceiveBeginPlay`)
  (set `self.Length_0` (- (`KismetArrayLibrary.Array_Length` (`self.MovePoint_0`)) 1))
  (set `self.TargetIndex_0` (`KismetMathLibrary.RandomIntegerInRange` 0 (`self.Length_0`))))

(event `self.ReceiveTick`
  (params (DeltaSeconds :type "Float (single-precision)"))
  (bind _output_location (`KismetMathLibrary.BreakTransform` (`|GetArrayItem` (`self.MovePoint_0`) (`self.TargetIndex_0`))))
  (bind _output_location_2 (`KismetMathLibrary.BreakTransform` (`|GetArrayItem` (`self.MovePoint_0`) (`self.TargetIndex_0`))))
  (`parent.ReceiveTick` DeltaSeconds)
  ;[1 1 1] 포인트에 착했다면
  (if (<= (`KismetMathLibrary.Vector_Distance` (`self.K2_GetActorLocation`) _output_location) 1.0)
    ;[1 1 1] 먼지를 쏜다
    (`self.Fire`)
    ;[1 1 1] 그리고 다음 타겟점을 정해줘
    (set `self.TargetIndex_0` (`KismetMathLibrary.RandomIntegerInRange` 0 (`self.Length_0`)))
    (else
      ;[1 1 1] 등속운동 P=P0+Vt
      (`self.K2_SetActorLocationAndRotation` (+ (`self.K2_GetActorLocation`) (* (* 0.0 (`self.MoveSpeed_0`)) (`KismetMathLibrary.Normal` (- _output_location_2 (`self.K2_GetActorLocation`)))))))))

(fn `UserConstructionScript`
  (`parent.UserConstructionScript`))