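; Actor that travels along the BoseSpline of a referenced track actor, matching its position and rotation.
; The Construction Script snaps it to the spline point chosen by PointIndex.
; On BeginPlay it passes Duration straight in as the timeline play rate, then calls MoveCube if ActiveCube is set.
; MoveCube plays a timeline whose alpha maps to distance over the full spline length, starting from zero.
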(event `MoveCube`
  (bind _returnvalue (`KismetMathLibrary.Lerp` 0.0 (`SplineComponent.GetSplineLength` (`/Game/JY/Blueprints/Spline_Track.BoseSpline` (`self.TrackRef`))) (`self.Alpha`)))
  ;[1 1 1] Comment
  (bind (_direction _alpha) (`Timeline|Timeline_CubeMover`)
    (:`Update`
      (set `self.Alpha` _alpha)
      (`self.K2_SetActorLocationAndRotation` (`SplineComponent.GetLocationAtDistanceAlongSpline` (`/Game/JY/Blueprints/Spline_Track.BoseSpline` (`self.TrackRef`)) _returnvalue "World") (`SplineComponent.GetRotationAtDistanceAlongSpline` (`/Game/JY/Blueprints/Spline_Track.BoseSpline` (`self.TrackRef`)) _returnvalue "World")))))

(event `self.ReceiveBeginPlay`
  ;[1 1 1] Comment
  (`TimelineComponent.SetPlayRate` (`self.Timeline_CubeMover`) (`self.Duration`))
  (if (`self.ActiveCube`)
    (`self.MoveCube`)))

(fn `UserConstructionScript`
  (bind _point_index (`self.Point Index`))
  (bind _bosespline (`/Game/JY/Blueprints/Spline_Track.BoseSpline` (`self.TrackRef`)))
  (`self.K2_SetActorLocationAndRotation` (`SplineComponent.GetLocationAtSplinePoint` _bosespline _point_index "World") (`SplineComponent.GetRotationAtSplinePoint` _bosespline _point_index "World")))