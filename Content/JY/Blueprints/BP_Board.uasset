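; BP_Board is a drawable whiteboard that accumulates marker strokes in the RT_Postit render target.
; BeginPlay creates a dynamic instance of M_Marker and clears the target to black.
; DrawOnWhiteBoard takes a 2D location, writes it to the material's "DrawLocattion" parameter and draws that material into the target.
; Tick passes delta time to a scalar parameter whose name is left as None.
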(event `self.ReceiveBeginPlay`
  (bind _returnvalue (`KismetMaterialLibrary.CreateDynamicMaterialInstance` "/Game/JY/Blueprints/M_Marker.M_Marker"))
  (set `self.White Board Marker` _returnvalue)
  (`KismetRenderingLibrary.ClearRenderTarget2D` "/Game/JY/Blueprints/RT_Postit.RT_Postit"))

(event `DrawOnWhiteBoard`
  (params (`Locationto Draw` :type "Vector2D Structure"))
  (bind _white_board_marker (`self.White Board Marker`))
  (`MaterialInstanceDynamic.SetVectorParameterValue` _white_board_marker "DrawLocattion" (`KismetMathLibrary.Conv_VectorToLinearColor` (`KismetMathLibrary.Conv_Vector2DToVector` `Locationto Draw` 0.1)))
  (`KismetRenderingLibrary.DrawMaterialToRenderTarget` "/Game/JY/Blueprints/RT_Postit.RT_Postit" _white_board_marker))

(event `self.ReceiveTick`
  (params (DeltaSeconds :type "Float (single-precision)"))
  (`MaterialInstanceDynamic.SetScalarParameterValue` (`self.White Board Marker`) "None" DeltaSeconds))

(fn `UserConstructionScript`)