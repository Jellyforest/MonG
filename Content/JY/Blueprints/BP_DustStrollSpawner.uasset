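; BP_DustStrollSpawner is a dust spawner, apparently for a boss, meant to wander between random MovePoints while firing dust.
; Tick moves it at constant speed to the target, then a two-second Timer gates random horizontal or vertical Arrow offsets and delayed Fire calls.
; ArrowMoveTimer should trigger retargeting, but it compares zero to MaxTime instead of its accumulated time, so the spawner never leaves its first point.
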(event `self.ReceiveBeginPlay`
  ;[1 1 1] 무브포인트를 랜덤으로 왔다갔다 했으면 좋겠다
  (set `self.Length` (- (`KismetArrayLibrary.Array_Length` (`self.MovePoint`)) 1))
  (set `self.TargetIndex` (`KismetMathLibrary.RandomIntegerInRange` 0 (`self.Length`))))

(event `self.ReceiveTick`
  (params (DeltaSeconds :type "Float (single-precision)"))
  (bind _output_location (`KismetMathLibrary.BreakTransform` (`|GetArrayItem` (`self.MovePoint`) (`self.TargetIndex`))))
  (bind _output_location_2 (`KismetMathLibrary.BreakTransform` (`|GetArrayItem` (`self.MovePoint`) (`self.TargetIndex`))))
  ;[1 1 1] 포인트에 착했다면
  (if (<= (`KismetMathLibrary.Vector_Distance` (`self.K2_GetActorLocation`) _output_location) 1.0)
    (bind _finish (`self.Timer` DeltaSeconds 2.0)) ; 타이머를 실행시켜줘
    (if _finish
      (bind _finish_2 (`self.ArrowMoveTimer` (`GameplayStatics.GetWorldDeltaSeconds`) 7.0)) ; arrow가 움직일 타이머
      (if _finish_2
        ;[1 1 1] 그리고 다음 타겟점을 정해줘
        (set `self.TargetIndex` (`KismetMathLibrary.RandomIntegerInRange` 0 (`self.Length`)))
        (else
          ;[1 1 1] 보스 안에 먼지스폰 arrow 랜덤으로 방향 설정
          (if (== (`KismetMathLibrary.RandomIntegerInRange` 0 1) 0)
            (`self.Horizontal Move` (`GameplayStatics.GetWorldDeltaSeconds`))
            ;[1 1 1] arrow 방향설정 후 그 축으로 움직여랏
            (`SceneComponent.K2_SetRelativeLocation` (`self.arrow`) (`KismetMathLibrary.MakeVector` (`self.VerticalMove`) (`self.HorizontalMove`)) false false :!label _label)
            ;[1 1 1] 100번 반복준비
            (for _ (range 2)
              ;[1 1 1] 딜레이 타이머
              (`KismetSystemLibrary.Delay` 1.0)
              ;[1 1 1] 먼지를 쏜다
              (`self.Fire`)
              (if true :!label _label_2
                _))
            (goto _label_2)
            (elif (== (`KismetMathLibrary.RandomIntegerInRange` 0 1) 1)
              (`self.Vertical Move` (`GameplayStatics.GetWorldDeltaSeconds`) 1.0)
              (goto _label))))))
    (else
      ;[1 1 1] 등속운동 P=P0+Vt
      (`self.K2_SetActorLocation` (+ (`self.K2_GetActorLocation`) (* (* (`GameplayStatics.GetWorldDeltaSeconds`) (`self.MoveSpeed`)) (`KismetMathLibrary.Normal` (- _output_location_2 (`self.K2_GetActorLocation`)))))))))

(fn `ArrowMoveTimer`
  (params (DeltaSec :type "Float (double-precision)") (MaxTime :type "Float (double-precision)"))
  (returns (Finish :type Boolean))
  (set `self.arrowCurTimer` (+ DeltaSec (`self.arrowCurTimer`)))
  (if (>= 0.0 MaxTime)
    (set `self.arrowCurTimer` 0.0)
    (return true)
    (else
      (return false))))

(fn `Horizontal Move`
  (params (DeltaSec :type "Float (double-precision)") (NewParam1 :type "Float (double-precision)"))
  (bind _returnvalue (* DeltaSec NewParam1))
  (bind _horizontalmove (`self.HorizontalMove`))
  (if (`self.isInc`)
    (bind _output_get (set `self.HorizontalMove` (+ _horizontalmove _returnvalue)))
    (if (>= _output_get 50.0)
      (set `self.isInc` false))
    (else
      (bind _output_get_2 (set `self.HorizontalMove` (- _horizontalmove _returnvalue)))
      (if (<= _output_get_2 -50.0)
        (set `self.isInc` true)))))

(fn `Timer`
  (params (DeltaSec :type "Float (double-precision)") (MaxTime :type "Float (double-precision)"))
  (returns (Finish :type Boolean))
  (locals (Count :type "Float (double-precision)" :default 0.0))
  (bind _output_get (set `self.TimerCount` (+ DeltaSec (`self.TimerCount`))))
  (if (>= _output_get MaxTime)
    (set `self.TimerCount` 0.0)
    (return true)
    (else
      (return false))))

(fn `UserConstructionScript`)

(fn `Vertical Move`
  (params (DeltaSec :type "Float (double-precision)") (NewParam1 :type "Float (double-precision)"))
  (bind _returnvalue (* DeltaSec NewParam1))
  (bind _verticalmove (`self.VerticalMove`))
  (set `self.VerticalMove` 0.0)
  (if (`self.isInc`)
    (bind _output_get (set `self.VerticalMove` (+ _verticalmove _returnvalue)))
    (if (>= _output_get 50.0)
      (set `self.isInc` false))
    (else
      (bind _output_get_2 (set `self.VerticalMove` (- _verticalmove _returnvalue)))
      (if (<= _output_get_2 -50.0)
        (set `self.isInc` true)))))