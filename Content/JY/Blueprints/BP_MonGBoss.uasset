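; BP_MonGBoss is a boss monster Blueprint that moves toward a target point.
; Each Tick it moves in a straight line at constant MoveSpeed toward MovePoint[TargetIndex], using a normalized direction scaled by delta time, without sweep.
; Movement stops only at zero distance, with no overshoot clamp.
; Nothing here changes TargetIndex, and a check of it against zero is left unconnected.
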(event `self.ReceiveTick`
  (params (DeltaSeconds :type "Float (single-precision)"))
  (bind _output_location (`KismetMathLibrary.BreakTransform` (`|GetArrayItem` (`self.MovePoint`) (`self.targetIndex`))))
  (bind _output_location_2 (`KismetMathLibrary.BreakTransform` (`|GetArrayItem` (`self.MovePoint`) (`self.TargetIndex`))))
  (if (not (<= (`KismetMathLibrary.Vector_Distance` (`self.K2_GetActorLocation`) _output_location) 0.0))
    ;[1 1 1] 등속운동 P=P0+Vt
    (`self.K2_SetActorLocation` (+ (`self.K2_GetActorLocation`) (* (* DeltaSeconds (`self.moveSpeed`)) (`KismetMathLibrary.Normal` (- _output_location_2 (`self.K2_GetActorLocation`))))))))

(fn `UserConstructionScript`)