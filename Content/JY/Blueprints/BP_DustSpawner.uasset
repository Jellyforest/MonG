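; BP_DustSpawner is an actor that wanders between the locations in its MovePoint array at constant speed.
; Each Tick it steps along the normalized direction to the target, then picks a random new index once within one unit.
; BeginPlay rolls the first index before Length is set from the array.
; Despite the name, the BP_Dust spawn and Fire call are disconnected, so it spawns nothing.
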(event `self.ReceiveBeginPlay`
  (set `self.TargetIndex` (`KismetMathLibrary.RandomIntegerInRange` 0 (`self.Length`)))
  (set `self.Length` (- (`KismetArrayLibrary.Array_Length` (`self.MovePoint`)) 1)))

(event `self.ReceiveTick`
  (params (DeltaSeconds :type "Float (single-precision)"))
  (bind _output_location (`KismetMathLibrary.BreakTransform` (`|GetArrayItem` (`self.MovePoint`) (`self.TargetIndex`))))
  (bind _output_location_2 (`KismetMathLibrary.BreakTransform` (`|GetArrayItem` (`self.MovePoint`) (`self.TargetIndex`))))
  (if (<= (`KismetMathLibrary.Vector_Distance` (`self.K2_GetActorLocation`) _output_location) 1.0)
    (set `self.TargetIndex` (`KismetMathLibrary.RandomIntegerInRange` 0 (`self.Length`)))
    (else
      ;[1 1 1] 등속운동 P=P0+Vt
      (`self.K2_SetActorLocationAndRotation` (+ (`self.K2_GetActorLocation`) (* (* DeltaSeconds (`self.MoveSpeed`)) (`KismetMathLibrary.Normal` (- _output_location_2 (`self.K2_GetActorLocation`)))))))))

(fn `UserConstructionScript`)